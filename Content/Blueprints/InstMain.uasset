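; InstMain holds a shared Players list of player info structs with a ready state, and offers a debug print helper.
; Events add a player, remove one by name, or update a player's Ready flag.
; Removal and ready updates locate entries through GetPlayerIndex, a linear name search returning Found and Index.
; PrintonLog joins two strings and prints them with configurable screen, log, color and duration.
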(event Custom|AddPlayer
  (params (NewPlayer :type Player%20Info%20Structure%20%28by%20ref%29))
  ;[1 1 1] Add Player
  (Utilities|Array|Add (Variables|Default|GetPlayers) NewPlayer))

(event Custom|RemovePlayer
  (params (PlayerName :type Text))
  (bind (_found _index) (CallFunction|GetPlayerIndex PlayerName))
  ;[1 1 1] Remove Player
  (if _found
    (Utilities|Array|RemoveIndex (Variables|Default|GetPlayers) _index)))

(event Custom|UpdatePlayerReady
  (params (PlayerName :type Text) (NewValue :type Boolean))
  (bind (_found _index) (CallFunction|GetPlayerIndex PlayerName))
  ;[1 1 1] Update Player Ready
  (if _found
    (Utilities|Struct|SetmembersinPlayerInfo (Utilities|Array|Get(acopy) (Variables|Default|GetPlayers) _index) NewValue)))

(event EventPrintonLog
  (params (String1 :type String) (String2 :type String) (bScreen :type Boolean) (bLog :type Boolean) (Color :type Color%20Structure) (Time :type Float%20%28single-precision%29))
  ;[1 1 1] Print On Log
  (Development|PrintString (Utilities|String|Append String1 String2) bScreen bLog (Math|Conversions|ToLinearColor(Color) Color) Time))

(fn GetPlayerIndex
  (params (PlayerName :type Text))
  (bind (_array_element _array_index) (Utilities|Array|ForEachLoopwithBreak (Variables|Default|GetPlayers) :!label _label)
    (:LoopBody
      (if (Utilities|Enum|Equal(Enum) (Utilities|Struct|BreakPlayerInfo _array_element) PlayerName)
        (LocalVariables|SetoutBool true)
        (LocalVariables|SetoutInt _array_index)
        (goto _label Break)))
    (:Completed
      (return (LocalVariables|GetoutBool) (LocalVariables|GetoutInt)))))