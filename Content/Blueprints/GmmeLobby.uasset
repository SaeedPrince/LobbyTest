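; GmmeLobby manages a multiplayer lobby roster, apparently as its game mode, tracking each player's name, host flag and ready state.
; A map links each PlayerController to its PlayerInfo, and every addition pushes the full list of infos to each controller's lobby widget.
; Ready changes remove the player's entry and re-add it with the new state, reusing the add event to refresh all widgets.
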(event Custom|UpdateUserWidgets
  (bind _mapplayercontrollerstoplayerinfos (Variables|Default|GetMapPlayerControllersToPlayerInfos))
  (bind _keys (Utilities|Map|Keys _mapplayercontrollerstoplayerinfos))
  (bind _values (Utilities|Map|Values _mapplayercontrollerstoplayerinfos))
  (for _array_element _keys
    (Default|UpdateLobbyWidget _array_element _values)))

(event Custom|AddPlayerInfo
  (params (PlayerController :type Plct%20Lobby%20Object%20Reference%20%28by%20ref%29) (PlayerInfo :type Player%20Info%20Structure%20%28by%20ref%29))
  (Utilities|Map|Add (Variables|Default|GetMapPlayerControllersToPlayerInfos) PlayerController PlayerInfo)
  (CallFunction|UpdateUserWidgets))

(event Custom|UpdateReadyState
  (params (inPlayerController :type Plct%20Lobby%20Object%20Reference) (inReady :type Boolean))
  (bind _mapplayercontrollerstoplayerinfos (Variables|Default|GetMapPlayerControllersToPlayerInfos))
  (bind _value (Utilities|Map|Find _mapplayercontrollerstoplayerinfos inPlayerController))
  (bind (_playername _bhost) (Utilities|Struct|BreakPlayerInfo _value))
  (Variables|Default|SetPlNm _playername)
  (Variables|Default|SetHst _bhost)
  (Utilities|Map|Remove _mapplayercontrollerstoplayerinfos inPlayerController)
  (CallFunction|AddPlayerInfo inPlayerController (Utilities|Struct|MakePlayerInfo (Variables|Default|GetPlNm) (Variables|Default|GetHst) inReady)))

(fn ConstructionScript)