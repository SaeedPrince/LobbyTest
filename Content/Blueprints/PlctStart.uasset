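; Player controller for the start screen that manages the start and lobby widgets and passes join requests on.
; On BeginPlay it shows the start widget only for the locally controlled player, whether client or listen-server host.
; Separate events remove that widget, add a non-host lobby widget, and forward a server name to the InstMain game instance to join.
; EndPlay removes all widgets.
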(event Custom|RemoveStartWidget
  ;[1 1 1] Remove Start Widget
  (Widget|RemovefromParent (Variables|Default|GetStartWidgetRef)))

(event Custom|AddLobbyWidget
  ;[1 1 1] Add lobby widget
  (bind _returnvalue (UserInterface|CreateWidget "/Game/Blueprints/WidgetLobby.WidgetLobby_C" self))
  (bind _output_get (Variables|Default|SetLobbyWidgetRef _returnvalue))
  (UserInterface|Viewport|AddtoViewport _output_get 0))

(event Custom|RequestJoinServer
  (params (inServerName :type Text%20%28by%20ref%29))
  ;[1 1 1] Request join server
  (bind _asinst_main (Utilities|Casting|CastToInstMain (Game|GetGameInstance)))
  (Class|GmInstMain|JoinServer _asinst_main inServerName))

(event EventBeginPlay
  (bind _returnvalue (Ability|HasAuthority))
  ;[1 1 1] Begin Play
  (if (or (not _returnvalue) (and _returnvalue (Pawn|IsLocalPlayerController)))
    (bind _returnvalue_2 (UserInterface|CreateWidget "/Game/Blueprints/WidgetStart.WidgetStart_C" self))
    (bind _output_get (Variables|Default|SetStartWidgetRef _returnvalue_2))
    (UserInterface|Viewport|AddtoViewport _output_get 0)))

(event EventEndPlay
  (params (EndPlayReason :type EEndPlayReason%20Enum :default "Destroyed"))
  ;[1 1 1] End Play
  (Viewport|RemoveAllWidgets))

(fn ConstructionScript)