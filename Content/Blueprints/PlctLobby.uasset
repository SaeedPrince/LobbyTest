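; Lobby player controller that shows the lobby widget, handles player joins and ready changes, and starts travel to the game map.
; BeginPlay creates the widget on clients and on the host's local controller, passing authority as the Host flag.
; Join and ready requests update the player list in the InstMain game instance, then refresh the widget slots; hosts join already ready.
; ServerTravel clears all widgets and runs a console command to load MapGame.
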(event Custom|RequestJoinPlayer
  (params (Player%20Name :type Text) (Host :type Boolean))
  (bind _asinst_main (Utilities|Casting|CastToInstMain (Game|GetGameInstance)))
  (Default|AddPlayer _asinst_main (Utilities|Struct|MakePlayerInfo Player%20Name Host Host))
  (CallFunction|UpdateAllWidgets (Variables|/Script/LobbyTest.GmInstMain|GetPlayers _asinst_main)))

(event Custom|UpdateAllWidgets
  (params (Players :type Array%20of%20Player%20Info%20Structures))
  (Default|UpdateSlots (Variables|Default|GetLobbyWidgetRef) Players))

(event Custom|RequestUpdateReady
  (params (PlayerName :type Text) (Ready :type Boolean))
  (bind _asinst_main (Utilities|Casting|CastToInstMain (Game|GetGameInstance)))
  (Default|UpdatePlayerReady _asinst_main PlayerName Ready)
  (CallFunction|UpdateAllWidgets (Variables|/Script/LobbyTest.GmInstMain|GetPlayers _asinst_main)))

(event Custom|ServerTravel
  (Viewport|RemoveAllWidgets)
  (Development|ExecuteConsoleCommand "ServerTravel MapGame" self))

(event EventBeginPlay
  (bind _returnvalue (Ability|HasAuthority))
  (if (or (not _returnvalue) (and _returnvalue (Pawn|IsLocalPlayerController)))
    (bind _returnvalue_2 (UserInterface|CreateWidget "/Game/Blueprints/WidgetLobby.WidgetLobby_C" self _returnvalue))
    (bind _output_get (Variables|Default|SetLobbyWidgetRef _returnvalue_2))
    (UserInterface|Viewport|AddtoViewport _output_get 0)))

(fn ConstructionScript)